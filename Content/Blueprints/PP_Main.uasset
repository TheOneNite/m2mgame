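; PP_Main is a camera-control Blueprint that pans the actor with the mouse and moves its camera vertically with the mousewheel.
; Tick adds scaled mouse-axis input to CameraX and CameraY, then shares CameraDrag's SetActorLocation, so panning runs every frame with Z fixed at zero.
; Mousewheel events step the Camera's relative Z up or down by CameraMoveZ, without clamping.
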(event EventTick
  (params (DeltaSeconds :type Float%20%28single-precision%29))
  (bind _output_get (Variables|Default|Setcamera_y (+ (Variables|Default|Getcamera_y) (* (Input|AxisValues|Getmouse_axis_y) (Variables|Default|Getcamera_move_y)))))
  (bind _output_get_2 (Variables|Default|Setcamera_x (+ (Variables|Default|Getcamera_x) (* (Input|AxisValues|Getmouse_axis_x) (Variables|Default|Getcamera_move_x)))))
  (Transformation|SetActorLocation (Math|Conversions|ToVector(Vector2D) (Math|Vector2D|MakeVector2D _output_get_2 _output_get)) false false))

(event EventCameraDrag
  (Transformation|SetActorLocation (Math|Conversions|ToVector(Vector2D) (Math|Vector2D|MakeVector2D (stale EventTick _output_get_2) (stale EventTick _output_get))) false false))

(event EventMousewheelDown
  (bind _camera (Variables|Default|GetCamera))
  (bind _returnvalue (Transformation|GetRelativeTransform _camera))
  (bind _location (Math|Transform|BreakTransform _returnvalue))
  (bind (_x _y _z) (Math|Vector|BreakVector _location))
  (Transformation|SetRelativeLocation _camera (Math|Vector|MakeVector _x _y (- _z (Variables|Default|Getcamera_move_z))) false false))

(event EventMousewheelUp
  (bind _camera (Variables|Default|GetCamera))
  (bind _returnvalue (Transformation|GetRelativeTransform _camera))
  (bind _location (Math|Transform|BreakTransform _returnvalue))
  (bind (_x _y _z) (Math|Vector|BreakVector _location))
  (Transformation|SetRelativeLocation _camera (Math|Vector|MakeVector _x _y (+ _z (Variables|Default|Getcamera_move_z))) false false))

(fn ConstructionScript)