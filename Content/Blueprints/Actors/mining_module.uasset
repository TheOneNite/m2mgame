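; Mining module for a building that sets up a mine location and previews the ground's average resource composition.
; DesignateMineLocation spawns an area cursor at the building, creates the resource widget and enters Setup, during which Tick recomputes the average and refreshes the widget.
; UpdateAvgComposition sphere-traces vertically around the cursor, with debug drawing, and averages GroundTile compositions per resource through running totals in BuildAvg, which are never cleared here.
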(event EventBeginPlay)

(event EventTick
  (params (DeltaSeconds :type Float%20%28single-precision%29))
  (switch Utilities|FlowControl|Switch|Switchonstatus_mining (Variables|Default|Getmine_status)
    (:NewEnumerator1
      (CallFunction|UpdateAvgComposition)
      (Default|UpdateComp (Variables|Default|GetwgAverageResources)))))

(event EventSelectActorComponent)

(fn DesignateMineLocation
  (bind _returnvalue (Game|SpawnActorfromClass "/Game/Blueprints/Actors/mining_cursor.mining_cursor_C" (Math|Conversions|ToTransform(Vector) (Transformation|GetActorLocation (Variables|Default|Getbuilding_ref))) "Undefined" 0 0))
  (Variables|Default|Setarea_cursor _returnvalue)
  (bind _returnvalue_2 (UserInterface|CreateWidget "/Game/UserInterfaces/mining_resources.mining_resources_C"))
  (bind _output_get (Variables|Default|SetwgAverageResources _returnvalue_2))
  (CallFunction|UpdateAvgComposition)
  (Variables|/Game/UserInterfaces/mining_resources.mining_resources_C|Setcomposition _output_get (Variables|Default|GetaverageComp))
  (Variables|Default|Setmine_status "NewEnumerator1"))

(fn UpdateAvgComposition
  (bind _area_cursor (Variables|Default|Getarea_cursor))
  (bind _build_avg (Variables|Default|Getbuild_avg))
  (bind _build_avg_2 (Variables|Default|Getbuild_avg))
  (bind _returnvalue (Transformation|GetActorLocation _area_cursor))
  (bind (_x _y _z) (Math|Vector|BreakVector _returnvalue))
  (bind _outhits (Collision|MultiSphereTraceByChannel (Math|Vector|MakeVector _x _y (+ _z 5e+02)) (Math|Vector|MakeVector _x _y (- _z 5e+02)) 4.5e+02 "TraceTypeQuery3" false 0 "ForDuration"))
  (for _array_element _outhits
    (bind _asground_tile (Utilities|Casting|CastToGroundTile (.HitActor (Collision|BreakHitResult _array_element))))
    (bind _keys (Utilities|Map|Keys (Variables|/Game/Blueprints/Actors/GroundTile.GroundTile_C|Getcomposition _asground_tile)))
    (for _array_element_2 _keys
      (Utilities|Map|Add _build_avg _array_element_2 (Utilities|Struct|Makebuild_average (+ (.value (.Value (Utilities|Map|Find _build_avg _array_element_2))) (.Value (Utilities|Map|Find (Variables|/Game/Blueprints/Actors/GroundTile.GroundTile_C|Getcomposition _asground_tile) _array_element_2))) (+ (.membercount (.Value (Utilities|Map|Find _build_avg _array_element_2))) 1.0))))
    (bind _keys_2 (Utilities|Map|Keys _build_avg_2))
    (for _array_element_3 _keys_2
      (Utilities|Map|Add (Variables|Default|GetaverageComp) _array_element_3 (/ (.value (.Value (Utilities|Map|Find _build_avg_2 _array_element_3))) (.membercount (.Value (Utilities|Map|Find _build_avg_2 _array_element_3))))))))