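; Citizen actor for a colony sim, simulating one inhabitant's survival needs and mental state.
; Each tick it breathes from suit or building oxygen and consumes carried or population food and water, dying from suffocation, thirst or starvation.
; Stress is a running average of living-space baseline and task modifier, raised by hunger and thirst.
; High stress randomly triggers breakdowns that remove it from its team until a random recovery returns it as unassigned.
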(event EventBeginPlay
  (Variables|Default|Setactive_task (Utilities|Struct|Maketask 0 "None"))
  (Utilities|FindIdleStress))

(event Collision|EventActorBeginOverlap
  (params (OtherActor :type Actor%20Object%20Reference)))

(event EventTick
  (params (DeltaSeconds :type Float%20%28single-precision%29))
  (CallFunction|LifeSupport (* DeltaSeconds (/ 1.0 24.0)))
  (CallFunction|StressTick))

(event EventDayOff
  (Variables|Default|Setactive_task (Utilities|Struct|Maketask (Variables|Default|Gethome) "None" 0.0)))

(fn ConstructionScript)

(fn LifeSupport
  (params (time :type Float%20%28single-precision%29))
  (bind _self self)
  (bind _pop_ref (Variables|Default|Getpop_ref))
  (bind _pop_ref_2 (Variables|Default|Getpop_ref))
  (bind _water_consumption (Variables|life_support|Getwater_consumption))
  (bind _food_consumption (Variables|life_support|Getfood_consumption))
  (Utilities|Breathe
    (:exhale
      (if (Variables|Default|Getoutside)
        (if (> (Variables|life_support|Getwater_bottle) 0.0)
          (Utilities|DecreDehydration)
          (Variables|life_support|Setwater_bottle (- (Variables|life_support|Getwater_bottle) 1.0))
          (else
            (Utilities|IncrementDehydration)))
        (elif (>= (Variables|/Game/Blueprints/Actors/population.population_C|Getwater _pop_ref_2) _water_consumption)
          (Utilities|DecreDehydration)
          (Variables|/Game/Blueprints/Actors/population.population_C|Setwater _pop_ref_2 (- (Variables|/Game/Blueprints/Actors/population.population_C|Getwater _pop_ref_2) _water_consumption))
          (else
            (Utilities|IncrementDehydration))))
      (if (Variables|Default|Getoutside)
        (if (> (Variables|life_support|Getlunchbox) 0.0)
          (Utilities|DecrementStarvation)
          (Variables|life_support|Setlunchbox (- (Variables|life_support|Getlunchbox) 1.0))
          (else
            (Utilities|IncrementStarvation)))
        (elif (>= (Variables|/Game/Blueprints/Actors/population.population_C|Getfood _pop_ref) _food_consumption)
          (Utilities|DecrementStarvation)
          (Variables|/Game/Blueprints/Actors/population.population_C|Setfood _pop_ref (- (Variables|/Game/Blueprints/Actors/population.population_C|Getfood _pop_ref) _food_consumption))
          (else
            (Utilities|IncrementStarvation))))
      (if (or (> (Variables|stress|Getdehydration) 5.0) (> (Variables|stress|Getstarvation) 25.0))
        (Utilities|Array|RemoveItem (Variables|/Game/Blueprints/Actors/team.team_C|Getmembers (Variables|Default|Getteam)) _self)
        (Utilities|Array|RemoveItem (Variables|/Game/Blueprints/Actors/population.population_C|Getcitizens (Variables|Default|Getpop_ref)) _self)
        (Actor|DestroyActor)))))

(fn StressTick
  (bind _stress_rate (Variables|stress|Getstress_rate))
  (bind _stress_rate_2 (Variables|stress|Getstress_rate))
  (bind _stress_rate_3 (Variables|stress|Getstress_rate))
  (bind _returnvalue (* _stress_rate 2.0))
  (if (Variables|stress|Getbreakdown)
    (Utilities|IsValid (Variables|Default|Getteam)
      (:Is%20Valid
        (Utilities|Array|RemoveItem (Variables|/Game/Blueprints/Actors/team.team_C|Getmembers (Variables|Default|Getteam)) self)
        (Variables|Default|Setteam 0)
        (Variables|Default|Setactive_task (Utilities|Struct|Maketask (Variables|Default|Gethome) "None")))
      (:Is%20Not%20Valid
        _))
    (bind _output_get (Variables|Default|Setstress_level (/ (+ (Variables|stress|Getidle_stress) (* (Variables|Default|Getstress_level) _returnvalue)) (+ _returnvalue 1.0))))
    (if (Math|Random|RandomBoolwithWeight (* (Math|Float|Clamp(Float) (- 1.0 _output_get) 0.0 2.0) 0.5))
      (Utilities|Array|Add (Variables|/Game/Blueprints/Actors/population.population_C|Getunassigned_citizens (Variables|Default|Getpop_ref)) self)
      (Variables|stress|Setbreakdown false))
    (else
      (if (== (.building (Utilities|Struct|Breaktask (Variables|Default|Getactive_task))) (Variables|Default|Gethome))
        (Variables|Default|Setstress_level (/ (+ (Variables|stress|Getidle_stress) (* (Variables|Default|Getstress_level) _stress_rate_3)) (+ _stress_rate_3 1.0))) ; new stress is average of old stresss*10 and new stress
        (else
          (Variables|Default|Setstress_level (/ (+ (* _stress_rate_2 (Variables|Default|Getstress_level)) (+ (.stress_mod (Utilities|Struct|Breaktask (Variables|Default|Getactive_task))) (Variables|stress|Getidle_stress))) (+ _stress_rate_2 1.0)))))
      (Variables|Default|Setstress_level (+ (+ (* (Variables|stress|Getstarvation) (Variables|life_support|Gethunger_factor)) (* (Variables|stress|Getdehydration) (Variables|life_support|Getthirst_factor))) (Variables|Default|Getstress_level)))
      (if (> (Variables|Default|Getstress_level) 1.0)
        (if (Math|Random|RandomBoolwithWeight (/ (- (Variables|Default|Getstress_level) 1.0) (Variables|stress|Getmental_stability))) ; roll for breakdown
          (Variables|stress|Setbreakdown true))))))