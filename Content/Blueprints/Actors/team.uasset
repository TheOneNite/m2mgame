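; Team actor that groups Members into a work crew, assigning them tasks from a queue or giving them days off.
; Each Tick counts days since the last break and checks size, destroying empty teams.
; A random roll weighted by average stress and break age decides between pushing the front task to members and registering with its building, or recomputing stress and resting.
; TaskDone clears the occupied flag and dequeues the task.
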(event EventBeginPlay)

(event Collision|EventActorBeginOverlap
  (params (OtherActor :type Actor%20Object%20Reference)))

(event EventTick
  (params (DeltaSeconds :type Float%20%28single-precision%29))
  (bind _task_queue (Variables|Default|Gettask_queue))
  (bind _output (Utilities|Array|Get(acopy) _task_queue))
  (bind (_building _skill) (Utilities|Struct|Breaktask _output))
  (Variables|Default|Setdays_since_break (+ (Variables|Default|Getdays_since_break) 1.0))
  (Utilities|CheckSize
    (:hires
      (if (> (Utilities|Array|Length (Variables|Default|Gettask_queue)) 0)
        (if (Math|Random|RandomBoolwithWeight (/ (- 1.0 (Variables|Default|Getaverage_stress)) (* (Variables|Default|Getdays_since_break) 0.1)))
          (if (and (Utilities|Name|Equal(Name) (.skill (Utilities|Struct|Breaktask (Variables|Default|Gettask_active))) _skill) (== (.building (Utilities|Struct|Breaktask (Variables|Default|Gettask_active))) _building))
            _
            (else
              (bind _output_get (Variables|Default|Settask_active _output))))
          (for _array_element (Variables|Default|Getmembers)
            (Variables|/Game/Blueprints/Actors/citizen.citizen_C|Setactive_task _array_element _output_get))
          (if (not (Variables|Default|Getis_research))
            (Utilities|Array|AddUnique (Variables|/Game/Blueprints/Actors/Building.Building_C|Getteams (.building (Variables|Default|Gettask_active))) self))
          (else
            (Utilities|GetAvrStress :!label _label
              (:NewParam2
                (for _array_element_2 (Variables|Default|Getmembers)
                  (Class|ITFPopulation|DayOff(Message) _array_element_2))
                (Variables|Default|Setdays_since_break 0.0)
                (Variables|Default|Setoccupied false)
                (Utilities|IsValid (.building (Variables|Default|Gettask_active))
                  (:Is%20Valid
                    (Utilities|Array|RemoveItem (Variables|/Game/Blueprints/Actors/Building.Building_C|Getteams (.building (Variables|Default|Gettask_active))) self)))))))
        (else
          (goto _label))))))

(event EventTaskDone
  (params (task :type Task%20Structure))
  (bind _task_queue (Variables|Default|Gettask_queue))
  (Variables|Default|Setoccupied false)
  (Utilities|IsValid (.building (Utilities|Struct|Breaktask task))
    (:Is%20Valid
      (Utilities|Array|RemoveItem _task_queue task))
    (:Is%20Not%20Valid
      (Utilities|Array|RemoveIndex _task_queue))))

(fn ConstructionScript)