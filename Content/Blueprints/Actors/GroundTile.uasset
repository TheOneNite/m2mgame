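; GroundTile is a terrain tile actor with a randomized resource composition and a dust, rock or ice type.
; Its construction script rolls dust or rock, then mineral amounts and rarer lodes from the Resource_composition table, plus latitude-weighted ice.
; InitializeTile makes latitude-weighted ice caps, spreading ice to neighbors by sphere trace, while BeginPlay applies dust and rock materials.
; SelectActor fills the player's UI with composition widgets, revealing contents only when Surveyed.
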(event EventBeginPlay
  (switch Utilities|FlowControl|Switch|Switchontile_enum (Utilities|Enum|ByteToEnumtile_enum (Variables|Default|Gettype))
    (:NewEnumerator0
      (Rendering|Material|SetMaterial (Variables|Default|GetTile) 0 "/Game/Graphics/Materials/mat_tile_sand.mat_tile_sand"))
    (:NewEnumerator1
      (Rendering|Material|SetMaterial (Variables|Default|GetTile) 0 "/Game/Graphics/Materials/mat_tile_rock.mat_tile_rock"))))

(event Collision|EventActorBeginOverlap
  (params (OtherActor :type Actor%20Object%20Reference)))

(event EventSelectActor
  (params (Player%20Controller :type Pc%20Main%20Object%20Reference))
  (bind _uimain_refpc (Variables|/Game/Blueprints/Pc_Main.Pc_Main_C|GetUIMain_RefPC Player%20Controller))
  (bind _composition (Variables|Default|Getcomposition))
  (if (Variables|Default|Getsurveyed)
    (bind _keys (Utilities|Map|Keys _composition))
    (for _array_element _keys
      (bind _returnvalue (UserInterface|CreateWidget "/Game/UserInterfaces/WG_composition_mat.WG_composition_mat_C"))
      (Variables|/Game/UserInterfaces/WG_composition_mat.WG_composition_mat_C|Setid _returnvalue _array_element)
      (Variables|/Game/UserInterfaces/WG_composition_mat.WG_composition_mat_C|Setqty _returnvalue (* (.Value (Utilities|Map|Find _composition _array_element)) 1e+02))
      (Variables|/Game/UserInterfaces/WG_composition_mat.WG_composition_mat_C|Settile _returnvalue self)
      (Widget|Panel|AddChild (Variables|/Game/UserInterfaces/UI_main.UI_Main_C|GetwrapBox_schemas _uimain_refpc) _returnvalue))
    (else
      (bind _keys_2 (Utilities|Map|Keys _composition))
      (for _array_element_2 _keys_2
        (bind _returnvalue_2 (UserInterface|CreateWidget "/Game/UserInterfaces/WG_composition_mat.WG_composition_mat_C"))
        (Variables|/Game/UserInterfaces/WG_composition_mat.WG_composition_mat_C|Settile _returnvalue_2 self)
        (Widget|Panel|AddChild (Variables|/Game/UserInterfaces/UI_main.UI_Main_C|GetwrapBox_schemas _uimain_refpc) _returnvalue_2)))))

(event EventTick
  (params (DeltaSeconds :type Float%20%28single-precision%29)))

(event EventInitializeTile
  (bind _returnvalue (Transformation|GetActorLocation))
  (bind _lat (Variables|Default|Getlat))
  (bind _returnvalue_2 (Math|Float|Absolute(Float) _lat))
  (if (Math|Random|RandomBoolwithWeight (Math|Float|Power (/ _returnvalue_2 1.3e+02) 4.0))
    (Utilities|Map|Add (Variables|Default|Getcomposition) "10" 0.95)
    (Variables|Default|Settype 2)
    (Rendering|Material|SetMaterial (Variables|Default|GetTile) 0 "/Game/Graphics/Materials/Mat_WhitePoly.Mat_WhitePoly")
    (bind _outhits (Collision|MultiSphereTraceByChannel _returnvalue _returnvalue (* _returnvalue_2 5.0) "TraceTypeQuery1" false 0 "None"))
    (for _array_element _outhits
      (bind _asground_tile (Utilities|Casting|CastToGroundTile (.HitActor (Collision|BreakHitResult _array_element))))
      (Variables|GroundTile_C|Settype _asground_tile 2)
      (Utilities|Map|Add (Variables|GroundTile_C|Getcomposition _asground_tile) "10" 0.95)
      (Rendering|Material|SetMaterial (Variables|GroundTile_C|GetTile _asground_tile) 0 "/Game/Graphics/Materials/Mat_WhitePoly.Mat_WhitePoly"))))

(fn ConstructionScript
  (bind _composition (Variables|Default|Getcomposition))
  (bind _composition_2 (Variables|Default|Getcomposition))
  (bind _composition_3 (Variables|Default|Getcomposition))
  (bind _composition_4 (Variables|Default|Getcomposition))
  (bind _composition_5 (Variables|Default|Getcomposition))
  (bind _composition_6 (Variables|Default|Getcomposition))
  (bind _composition_7 (Variables|Default|Getcomposition))
  (bind _composition_8 (Variables|Default|Getcomposition))
  (bind _composition_9 (Variables|Default|Getcomposition))
  (bind _composition_10 (Variables|Default|Getcomposition))
  (if (Math|Random|RandomBoolwithWeight 0.2)
    (bind _returnvalue (Utilities|GetDataTableRow "/Game/Tables/resource_composition.resource_composition" "base_rock")
      (:then
        (Utilities|Map|Add _composition "2" (Math|Random|RandomFloatinRange (.nitrogen_low (Utilities|Struct|Breakcomposition _returnvalue)) (.nitrogen_high (Utilities|Struct|Breakcomposition _returnvalue))))
        (Utilities|Map|Add _composition "4" (Math|Random|RandomFloatinRange (.sulpher_low (Utilities|Struct|Breakcomposition _returnvalue)) (.sulpher_high (Utilities|Struct|Breakcomposition _returnvalue))))
        (Utilities|Map|Add _composition "3" (Math|Random|RandomFloatinRange (.silica_low (Utilities|Struct|Breakcomposition _returnvalue)) (.silica_high (Utilities|Struct|Breakcomposition _returnvalue))))
        (Utilities|Map|Add _composition "7" (Math|Random|RandomFloatinRange (.halogens_low (Utilities|Struct|Breakcomposition _returnvalue)) (.halogens_high (Utilities|Struct|Breakcomposition _returnvalue))))
        (Variables|Default|Settype 1)
        (bind _returnvalue_2 (Utilities|GetDataTableRow "/Game/Tables/resource_composition.resource_composition" "base_rock")
          (:then
            (Utilities|Map|Add _composition_2 "0" (Math|Random|RandomFloatinRange (.iron_low (Utilities|Struct|Breakcomposition _returnvalue_2)) (.iron_high (Utilities|Struct|Breakcomposition _returnvalue_2))))
            (if (Math|Random|RandomBoolwithWeight 0.15) ; iron deposit roll
              (bind _returnvalue_3 (Utilities|GetDataTableRow "/Game/Tables/resource_composition.resource_composition" "rock_lode_mods")
                (:then
                  (Utilities|Map|Add _composition_2 "0" (* (Math|Random|RandomFloatinRange (.iron_low (Utilities|Struct|Breakcomposition _returnvalue_3)) (.iron_high (Utilities|Struct|Breakcomposition _returnvalue_3))) (.Value (Utilities|Map|Find _composition_5 "0")))))))
            (if (Math|Random|RandomBoolwithWeight 0.05) ; RE deposit roll
              (Utilities|Map|Add _composition_5 "2" (Math|Random|RandomFloatinRange (.Re_low (Utilities|Struct|Breakcomposition _returnvalue_2)) (.RE_high (Utilities|Struct|Breakcomposition _returnvalue_2))))
              (if (Math|Random|RandomBoolwithWeight 0.3) ; RE lode roll
                (Utilities|Map|Add _composition_5 "2" (* (.Value (Utilities|Map|Find _composition_5 "2")) (Math|Random|RandomFloatinRange (.Re_low (Utilities|Struct|Breakcomposition _returnvalue_3)) (.RE_high (Utilities|Struct|Breakcomposition _returnvalue_3)))))))
            (Utilities|Map|Add _composition_10 "1" (Math|Random|RandomFloatinRange (.al_low (Utilities|Struct|Breakcomposition _returnvalue_2)) (.al_high (Utilities|Struct|Breakcomposition _returnvalue_2))))
            (if (Math|Random|RandomBoolwithWeight 0.3) ; AL lode roll
              (Utilities|Map|Add _composition_10 "1" (* (.Value (Utilities|Map|Find _composition_10 "1")) (Math|Random|RandomFloatinRange (.al_low (Utilities|Struct|Breakcomposition _returnvalue_3)) (.al_high (Utilities|Struct|Breakcomposition _returnvalue_3))))))
            (bind _keys (Utilities|Map|Keys _composition_7))
            (for _array_element _keys
              (Variables|Default|Setresource_percent (+ (Variables|Default|Getresource_percent) (.Value (Utilities|Map|Find _composition_6 _array_element)))))
            (Utilities|Map|Add _composition_6 "8" (- 1.0 (Variables|Default|Getresource_percent)))))))
    (else
      (bind _returnvalue_4 (Utilities|GetDataTableRow "/Game/Tables/resource_composition.resource_composition" "base_dust")
        (:then
          (Utilities|Map|Add _composition_4 "7" (Math|Random|RandomFloatinRange (.halogens_low (Utilities|Struct|Breakcomposition _returnvalue_4)) (.halogens_high (Utilities|Struct|Breakcomposition _returnvalue_4))))
          (Utilities|Map|Add _composition_4 "3" (Math|Random|RandomFloatinRange (.silica_low (Utilities|Struct|Breakcomposition _returnvalue_4)) (.silica_high (Utilities|Struct|Breakcomposition _returnvalue_4))))
          (Utilities|Map|Add _composition_4 "4" (Math|Random|RandomFloatinRange (.sulpher_low (Utilities|Struct|Breakcomposition _returnvalue_4)) (.sulpher_high (Utilities|Struct|Breakcomposition _returnvalue_4))))
          (Utilities|Map|Add _composition_4 "2" (Math|Random|RandomFloatinRange (.nitrogen_low (Utilities|Struct|Breakcomposition _returnvalue_4)) (.nitrogen_high (Utilities|Struct|Breakcomposition _returnvalue_4))))
          (Utilities|Map|Add _composition_4 "8" (Math|Random|RandomFloatinRange (.rock_low (Utilities|Struct|Breakcomposition _returnvalue_4)) (.rock_high (Utilities|Struct|Breakcomposition _returnvalue_4))))
          (Utilities|Map|Add _composition_4 "10" (Math|Random|RandomFloatinRange (.water_low (Utilities|Struct|Breakcomposition _returnvalue_4)) (.water_high (Utilities|Struct|Breakcomposition _returnvalue_4))))
          (Variables|Default|Settype 0)
          (bind _returnvalue_5 (Utilities|GetDataTableRow "/Game/Tables/resource_composition.resource_composition" "base_dust")
            (:then
              (Utilities|Map|Add _composition_8 "0" (Math|Random|RandomFloatinRange (.iron_low (Utilities|Struct|Breakcomposition _returnvalue_5)) (.iron_high (Utilities|Struct|Breakcomposition _returnvalue_5))))
              (if (Math|Random|RandomBoolwithWeight 0.15) ; iron deposit roll
                (bind _returnvalue_6 (Utilities|GetDataTableRow "/Game/Tables/resource_composition.resource_composition" "dust_lode_mods")
                  (:then
                    (Utilities|Map|Add _composition_8 "0" (* (Math|Random|RandomFloatinRange (.iron_low (Utilities|Struct|Breakcomposition _returnvalue_6)) (.iron_high (Utilities|Struct|Breakcomposition _returnvalue_6))) (.Value (Utilities|Map|Find _composition_9 "0")))))))
              (if (Math|Random|RandomBoolwithWeight 0.05) ; RE deposit roll
                (Utilities|Map|Add _composition_9 "2" (Math|Random|RandomFloatinRange (.Re_low (Utilities|Struct|Breakcomposition _returnvalue_5)) (.RE_high (Utilities|Struct|Breakcomposition _returnvalue_5))))
                (if (Math|Random|RandomBoolwithWeight 0.1) ; RE lode roll
                  (Utilities|Map|Add _composition_9 "2" (* (.Value (Utilities|Map|Find _composition_9 "2")) (Math|Random|RandomFloatinRange (.Re_low (Utilities|Struct|Breakcomposition _returnvalue_6)) (.RE_high (Utilities|Struct|Breakcomposition _returnvalue_6)))))))
              (Utilities|Map|Add _composition_3 "1" (Math|Random|RandomFloatinRange (.al_low (Utilities|Struct|Breakcomposition _returnvalue_5)) (.al_high (Utilities|Struct|Breakcomposition _returnvalue_5))))
              (if (Math|Random|RandomBoolwithWeight 0.15) ; iron deposit roll
                (Utilities|Map|Add _composition_3 "1" (* (Math|Random|RandomFloatinRange (.al_low (Utilities|Struct|Breakcomposition _returnvalue_6)) (.al_high (Utilities|Struct|Breakcomposition _returnvalue_6))) (.Value (Utilities|Map|Find _composition_3 "1")))))
              (bind _keys_2 (Utilities|Map|Keys _composition_7))
              (for _array_element_2 _keys_2
                (Variables|Default|Setresource_percent (+ (.Value (Utilities|Map|Find _composition_6 _array_element_2)) (Variables|Default|Getresource_percent))))
              (Utilities|Map|Add _composition_6 "9" (- 1.0 (Variables|Default|Getresource_percent)))))))))
  (if (Math|Random|RandomBoolwithWeight (/ (Math|Float|Absolute(Float) (Variables|Default|Getlat)) 9e+01))
    (Utilities|Map|Add (Variables|Default|Getcomposition) "2" 0.95)
    (Variables|Default|Settype 2)
    (Rendering|Material|SetMaterial (Variables|Default|GetTile) 0 "/Game/Graphics/Materials/Mat_WhitePoly.Mat_WhitePoly")))