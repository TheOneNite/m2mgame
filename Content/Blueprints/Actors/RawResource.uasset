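; RawResource is a resource actor whose Model mesh scales uniformly with its quantity, clamped between zero and full size.
; On BeginPlay it adds itself to LinkedResources.
; Each Tick, any rise in Quantity sets a per-frame step of one thirtieth of the gain, which accumulates into VisualQuantity to drive the scale.
; The step is frame-based and never reset here, and decreases in Quantity leave it unchanged.
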(event EventBeginPlay
  (Utilities|Array|Add (Variables|Default|Getlinked_resources) self))

(event EventTick
  (params (DeltaSeconds :type Float%20%28single-precision%29))
  (if (> (- (Variables|Default|GetQuantity) (Variables|Default|Getold_quant)) 0.0)
    (Variables|Default|Setresize_smoothing (/ (- (Variables|Default|GetQuantity) (Variables|Default|Getold_quant)) 3e+01))
    (Variables|Default|Setold_quant (Variables|Default|GetQuantity)))
  (Variables|Default|Setvisual_quantity (+ (Variables|Default|Getvisual_quantity) (Variables|Default|Getresize_smoothing)))
  (Transformation|SetWorldScale3D (Variables|Default|Getmodel) (Math|Vector|MakeVector (Math|Float|Clamp(Float) (/ (Variables|Default|Getvisual_quantity) 6e+02) 0.0 1.0) (Math|Float|Clamp(Float) (/ (Variables|Default|Getvisual_quantity) 6e+02) 0.0 1.0) (Math|Float|Clamp(Float) (/ (Variables|Default|Getvisual_quantity) 6e+02) 0.0 1.0))))

(fn ConstructionScript)