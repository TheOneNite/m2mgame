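; Placement cursor actor for choosing the ground tiles that a source building will mine.
; Every tick it teleports to the hit point under the player's mouse cursor.
; A primed left-click release capsule-traces downward, collects GroundTiles matching the target type, passes them with the schema ID to the building's MiningOpenSetup, then destroys the cursor.
; Releasing the right mouse button destroys it without making a selection.
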(event EventBeginPlay)

(event Collision|EventActorBeginOverlap
  (params (OtherActor :type Actor%20Object%20Reference)))

(event EventTick
  (params (DeltaSeconds :type Float%20%28single-precision%29))
  (Transformation|SetActorLocation (.Location (Collision|BreakHitResult (.HitResult (Game|Player|GetHitResultUnderCursorbyChannel (Variables|Default|GetPC_main) "TraceTypeQuery3" true)))) false true))

(event Input|MouseEvents|RightMouseButton
  (params (Key :type Key%20Structure :default "AnyKey"))
  (:Released
    (Actor|DestroyActor)))

(event Input|MouseEvents|LeftMouseButton
  (params (Key :type Key%20Structure :default "AnyKey"))
  (bind _returnvalue (Transformation|GetActorLocation))
  (bind _selectedtiles (Variables|Default|GetselectedTiles))
  (bind (_x _y) (Math|Vector|BreakVector _returnvalue))
  (:Pressed
    (bind _output_get (Variables|Default|Setprimer true)))
  (:Released
    (if _output_get
      (bind _outhits (Class|KismetSystemLibrary|CapsuleTraceMulti _returnvalue (Math|Vector|MakeVector _x _y -5e+01) 2.5e+02 1e+01 "TraceTypeQuery4" false 0 "None" true))
      (for _array_element _outhits
        (bind _asground_tile (Utilities|Casting|CastToGroundTile (.HitActor (Collision|BreakHitResult _array_element)))
          (:then
            (if (== (Variables|/Game/Blueprints/Actors/GroundTile.GroundTile_C|Gettype _asground_tile) (Variables|Default|GettargetTileType))
              (Utilities|Array|AddUnique _selectedtiles _asground_tile)
              (Development|PrintString (Utilities|GetDisplayName _asground_tile))))
          (:CastFailed
            (Development|PrintString "notatile"))))
      (Default|MiningOpenSetup (Variables|Default|GetsourceBuilding) _selectedtiles (Variables|Default|GetschemaId) (Variables|Default|GettargetTileType))
      (Actor|DestroyActor))))

(fn ConstructionScript)