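; Player controller for a tile-based building game, handling mouse and key input, building placement, landing-site selection and HUD panels.
; A ControlMode state machine sets the cursor and routes clicks to selection, targeting, construction or global view, messaging the selected actor or pawn.
; Shift-click chains building placements.
; Global clicks store coordinates in the game instance, while selections fill UI_Main with building materials, components, inventory, resources and construction category buttons.
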(event EventSpawnResourceUI
  (params (resource_connected :type Building%20Object%20Reference))
  ;[1 1 1] UI for resource/material/component Quantity
)

(event EventTick
  (params (DeltaSeconds :type Float%20%28single-precision%29))
  (switch Utilities|FlowControl|Switch|Switchoncontrol_modes_enum (Variables|Default|GetControlMode)
    (:NewEnumerator0
      (Variables|Default|SetCurrentMouseCursor "Default" :!label _label))
    (:NewEnumerator1
      (Variables|Default|SetCurrentMouseCursor "Crosshairs" :!label _label_2))
    (:NewEnumerator2
      (goto _label_2))
    (:NewEnumerator3
      (goto _label))
    (:NewEnumerator4
      (Variables|Default|SetCurrentMouseCursor "None"))
    (:NewEnumerator5
      (goto _label_2))
    (:NewEnumerator6
      (goto _label))))

(event EventDesignateStorageMode
  ;[1 1 1] Change to storage tile designate input mode from message
  (Variables|Default|SetControlMode "NewEnumerator0"))

(event EventSpawnBuildingUI
  (params (Building :type Building%20Object%20Reference))
  (bind _uimain_refpc (Variables|Default|GetUIMain_RefPC))
  (bind _uimain_refpc_2 (Variables|Default|GetUIMain_RefPC))
  (bind _uimain_refpc_3 (Variables|Default|GetUIMain_RefPC))
  (bind _inventory (Variables|/Game/Blueprints/Actors/Building.Building_C|GetInventory Building))
  (bind _verticalbox_components (Variables|/Game/UserInterfaces/UI_main.UI_Main_C|GetVerticalBox_components _uimain_refpc_3))
  (bind _verticalbox_materials (Variables|/Game/UserInterfaces/UI_main.UI_Main_C|GetVerticalBox_Materials _uimain_refpc_2))
  (bind _scrollbox_inventory (Variables|/Game/UserInterfaces/UI_main.UI_Main_C|GetScrollBox_Inventory _uimain_refpc))
  ;[1 1 1] UI for resource/material/component Quantity
  (Utilities|FlowControl|Sequence
    (:then_0
      (Widget|Panel|ClearChildren _verticalbox_materials)
      (Widget|SetVisibility (Variables|/Game/UserInterfaces/UI_main.UI_Main_C|GetHorizontalBox_Materials _uimain_refpc_2) "Visible")
      (bind _keys (Utilities|Map|Keys (Variables|/Game/Blueprints/Actors/Building.Building_C|GetMaterials Building)))
      (for (_array_element _array_index) _keys
        (bind _returnvalue (UserInterface|CreateWidget "/Game/UserInterfaces/WG_counter_mat.WG_counter_mat_C" self))
        (Variables|/Game/UserInterfaces/WG_counter_mat.WG_counter_mat_C|Setselected_building _returnvalue Building)
        (Variables|/Game/UserInterfaces/WG_counter_mat.WG_counter_mat_C|Setid _returnvalue _array_element)
        (Variables|/Game/UserInterfaces/WG_counter_mat.WG_counter_mat_C|SetIndex _returnvalue _array_index)
        (Widget|Panel|AddChild _verticalbox_materials _returnvalue)))
    (:then_1
      (Widget|Panel|ClearChildren _verticalbox_components)
      (Widget|SetVisibility (Variables|/Game/UserInterfaces/UI_main.UI_Main_C|GetHorizontalBox_Components _uimain_refpc_3) "Visible")
      (bind _keys_2 (Utilities|Map|Keys (Variables|/Game/Blueprints/Actors/Building.Building_C|GetComponents Building)))
      (for _array_element_2 _keys_2
        (bind _returnvalue_2 (UserInterface|CreateWidget "/Game/UserInterfaces/WG_Components.WG_Components_C" self))
        (Variables|/Game/UserInterfaces/WG_Components.WG_Components_C|SetOwningBuilding _returnvalue_2 Building)
        (Variables|/Game/UserInterfaces/WG_Components.WG_Components_C|Setid _returnvalue_2 _array_element_2)
        (Widget|Panel|AddChild _verticalbox_components _returnvalue_2)))
    (:then_2
      (Widget|Panel|ClearChildren _scrollbox_inventory)
      (Widget|SetVisibility (Variables|/Game/UserInterfaces/UI_main.UI_Main_C|GetHorizontalBox_Inventory _uimain_refpc) "Visible")
      (bind _keys_3 (Utilities|Map|Keys _inventory))
      (for _array_element_3 _keys_3
        (bind _returnvalue_3 (UserInterface|CreateWidget "/Game/UserInterfaces/WG_Inventory.WG_Inventory_C" self))
        (Variables|/Game/UserInterfaces/WG_Inventory.WG_Inventory_C|SetOwningBuilding _returnvalue_3 Building)
        (Variables|/Game/UserInterfaces/WG_Inventory.WG_Inventory_C|Setid _returnvalue_3 _array_element_3)
        (Variables|/Game/UserInterfaces/WG_Inventory.WG_Inventory_C|Setqty _returnvalue_3 (.Value (Utilities|Map|Find _inventory _array_element_3)))
        (Class|ITFUI|DefineButton(Message) _returnvalue_3)
        (Widget|Panel|AddChild _scrollbox_inventory _returnvalue_3)))
    (:then_3
      (CallFunction|CreateResourceUi Building)
      (Development|SetHiddeninGame (Variables|/Game/Blueprints/Actors/Building.Building_C|Getselection_ring Building) true false))))

(event EventBeginPlay
  ;[1 1 1] Begin play make mouse visible
  (Variables|Default|SetbShowMouseCursor true)
  (bind _aspp_main (Utilities|Casting|CastToPP_Main (Pawn|GetControlledPawn)))
  (Variables|Default|Setctrl_pawn _aspp_main)
  (bind _returnvalue (Game|GetCurrentLevelName true))
  (Development|PrintString _returnvalue)
  (if (Utilities|Enum|Equal(Enum) _returnvalue "Landing_selection")
    (bind _output_get (Variables|Default|SetControlMode "NewEnumerator6"))
    (Development|PrintString (Utilities|String|EnumtoString _output_get))
    (else
      (Variables|Default|SetControlMode "NewEnumerator0"))))

(event Input|KeyboardEvents|F10
  (params (Key :type Key%20Structure :default "AnyKey"))
  (:Released
    (bind _returnvalue (UserInterface|CreateWidget "/Game/UserInterfaces/MainMenuUI/Menu_ingame.Menu_ingame_C" self))
    (UserInterface|Viewport|AddtoViewport _returnvalue 0)))

(event Input|MouseEvents|ShiftLeftMouseButton
  (params (Key :type Key%20Structure :default "AnyKey"))
  (bind _self self)
  (bind _self_2 self)
  (bind (_locationx _locationy) (Class|WidgetLayoutLibrary|GetMousePositionScaledbyDPI _self))
  (:Released
    (switch Utilities|FlowControl|Switch|Switchoncontrol_modes_enum (Variables|Default|GetControlMode)
      (:NewEnumerator4
        (CallFunction|PlaceBuilding)
        (bind _returnvalue (Game|SpawnActorfromClass "/Game/Blueprints/Actors/Building.Building_C" (Math|Conversions|ToTransform(Vector) (Math|Conversions|ToVector(Vector2D) (Math|Vector2D|MakeVector2D _locationx _locationy))) "AlwaysSpawn" 0 0))
        (Variables|/Game/Blueprints/Actors/Building.Building_C|Setid _returnvalue (Variables|/Game/Blueprints/Actors/Building.Building_C|Getid (Variables|Default|Getconstruction_building)))
        (bind _returnvalue_2 (Utilities|GetDataTableRow "/Game/Tables/Buildings/buildings_basic.buildings_basic" (Variables|/Game/Blueprints/Actors/Building.Building_C|Getid (Variables|Default|Getconstruction_building)))
          (:then
            (Components|StaticMesh|SetStaticMesh (Variables|/Game/Blueprints/Actors/Building.Building_C|GetBuildingModel _returnvalue) (.model (Utilities|Struct|Breakbuildings_basic_struct _returnvalue_2)))
            (Rendering|Material|SetMaterial (Variables|/Game/Blueprints/Actors/Building.Building_C|GetBuildingModel _returnvalue) 0 "/Game/Graphics/Meshes/Material_001.Material_001")
            (Variables|/Game/Blueprints/Actors/Building.Building_C|Setowning_pc _returnvalue _self_2)
            (Variables|Pc_Main_C|Setconstruction_building _self_2 _returnvalue)
            (Collision|SetActorEnableCollision _returnvalue false)
            (Variables|Pc_Main_C|SetControlMode _self_2 "NewEnumerator4")))))))

(event Input|MouseEvents|LeftMouseButton
  (params (Key :type Key%20Structure :default "AnyKey"))
  (bind _hitresult (Game|Player|GetHitResultUnderCursorbyChannel "TraceTypeQuery3" true))
  (bind _hitactor (Collision|BreakHitResult _hitresult))
  ;[1 1 1] Left mouse button
  (:Released
    (Development|PrintString (Utilities|String|EnumtoString (Variables|Default|GetControlMode)))
    (switch Utilities|FlowControl|Switch|Switchoncontrol_modes_enum (Variables|Default|GetControlMode)
      (:NewEnumerator0
        ;[1 1 1] Normal mouse command
        (Utilities|ClearStockpileUI
          (:Out
            (Utilities|IsValid (Variables|Default|GetSelectedActor)
              (:Is%20Valid
                (Class|ITFUI|UnselectActor(Message) (Variables|Default|GetSelectedActor)))
              (:Is%20Not%20Valid
                _))
            (bind _output_get (Variables|Default|SetSelectedActor (.HitActor (Collision|BreakHitResult (.HitResult (Game|Player|GetHitResultUnderCursorbyChannel "TraceTypeQuery3" true))))))
            (Class|ITFUI|SelectActor(Message) _output_get self)
            (Utilities|Casting|CastToGroundTile _output_get
              (:then
                (CallFunction|CreateConstructionButtons))
              (:CastFailed
                _))
            (Widget|Panel|ClearChildren (Variables|/Game/UserInterfaces/UI_main.UI_Main_C|Getinstruction_box (Variables|Default|GetUIMain_RefPC))))))
      (:NewEnumerator1
        (CallFunction|TargetTile))
      (:NewEnumerator2
        (bind _asground_tile (Utilities|Casting|CastToGroundTile (.HitActor (Collision|BreakHitResult (.HitResult (Game|Player|GetHitResultUnderCursorbyChannel "TraceTypeQuery3" true)))))
          (:then
            (Class|ITFStockpiles|TargetTile(Message) (Variables|Default|GetSelectedActor) _asground_tile))
          (:CastFailed
            (Development|PrintString "could not find tile"))))
      (:NewEnumerator3
        (Variables|Default|SetControlMode "NewEnumerator0"))
      (:NewEnumerator4
        (CallFunction|PlaceBuilding))
      (:NewEnumerator5
        (Class|ITFStockpiles|TargetActor(Message) (Variables|Default|GetSelectedActor) _hitactor)
        (Variables|Default|SetControlMode "NewEnumerator0"))
      (:NewEnumerator6
        (CallFunction|GlobalClick))
      (:NewEnumerator7
        (Class|ITFUI|UiTargetActor(Message) (Variables|Default|Getrequesting_ui) _hitactor)
        (Variables|Default|SetControlMode "NewEnumerator3")))))

(event Input|MouseEvents|MouseWheelUp
  (params (Key :type Key%20Structure :default "AnyKey"))
  (:Released
    (Class|ITFUI|MousewheelUp(Message) (Variables|Default|Getctrl_pawn))))

(event Input|MouseEvents|MouseWheelDown
  (params (Key :type Key%20Structure :default "AnyKey"))
  (:Released
    (Class|ITFUI|MousewheelDown(Message) (Variables|Default|Getctrl_pawn))))

(event Input|MouseEvents|RightMouseButton
  (params (Key :type Key%20Structure :default "AnyKey"))
  (bind _ctrl_pawn (Variables|Default|Getctrl_pawn))
  (:Pressed
    (switch Utilities|FlowControl|Switch|Switchoncontrol_modes_enum (Variables|Default|GetControlMode)
      (:NewEnumerator0
        (Actor|Tick|SetActorTickEnabled _ctrl_pawn true))))
  (:Released
    (switch Utilities|FlowControl|Switch|Switchoncontrol_modes_enum (Variables|Default|GetControlMode)
      (:NewEnumerator0
        (Actor|Tick|SetActorTickEnabled _ctrl_pawn))
      (:NewEnumerator1
        (Variables|Default|SetControlMode "NewEnumerator0" :!label _label))
      (:NewEnumerator2
        (goto _label))
      (:NewEnumerator3
        (goto _label))
      (:NewEnumerator4
        (Actor|DestroyActor (Variables|Default|Getconstruction_building))
        (goto _label))
      (:NewEnumerator5
        (goto _label)))))

(event Input|KeyboardEvents|H
  (params (Key :type Key%20Structure :default "AnyKey"))
  (bind _uimain_refpc (Variables|Default|GetUIMain_RefPC))
  (:Pressed
    (Utilities|MainUiControl
      (:Out
        (bind _returnvalue (UserInterface|CreateWidget "/Game/UserInterfaces/SlotInventorySystem/WG_InventoryMain.WG_InventoryMain_C"))
        (Default|SpawnWGInventoryMain _returnvalue 4 4)
        (Widget|Panel|AddChild (Variables|/Game/UserInterfaces/UI_main.UI_Main_C|GetSizeBox_CenterInterface _uimain_refpc) _returnvalue)
        (Widget|SetVisibility (Variables|/Game/UserInterfaces/UI_main.UI_Main_C|GetVerticalBox_CentralInterface _uimain_refpc) "Visible")))))

(event Input|KeyboardEvents|Escape
  (params (Key :type Key%20Structure :default "AnyKey"))
  (:Pressed
    (Variables|Default|SetControlMode "NewEnumerator0")))

(fn ConstructionScript
  (Variables|Default|SetbShowMouseCursor true))

(fn PlaceBuilding
  (bind _construction_building (Variables|Default|Getconstruction_building))
  (Variables|/Game/Blueprints/Actors/Building.Building_C|Setpop_ref _construction_building (Variables|Default|Getpop_ref))
  (Collision|SetActorEnableCollision _construction_building true)
  (Default|ScaleBuilding _construction_building)
  (Variables|/Game/Blueprints/Actors/Building.Building_C|Setconstruction_status _construction_building "NewEnumerator1")
  (Default|BeginConstruction _construction_building)
  (Variables|Default|SetControlMode "NewEnumerator0"))

(fn CreateConstructionButtons
  (bind _self self)
  (for _index (range 0 4)
    (bind _returnvalue (UserInterface|CreateWidget "/Game/UserInterfaces/WG_button_building_category.WG_button_building_category_C" _self))
    (Variables|/Game/UserInterfaces/WG_button_building_category.WG_button_building_category_C|Setpc_ref _returnvalue _self)
    (Variables|/Game/UserInterfaces/WG_button_building_category.WG_button_building_category_C|Settype _returnvalue (Utilities|Enum|ByteToEnumbuilding_categories (Math|Conversions|ToByte(Integer) _index)))
    (Variables|/Game/UserInterfaces/WG_button_building_category.WG_button_building_category_C|Setpop_ref _returnvalue (Variables|Default|Getpop_ref))
    (Widget|Panel|AddChild (Variables|/Game/UserInterfaces/UI_main.UI_Main_C|Gethorbox_buttons (Variables|Default|GetUIMain_RefPC)) _returnvalue)))

(fn TargetTile
  (bind _asground_tile (Utilities|Casting|CastToGroundTile (.HitActor (Collision|BreakHitResult (.HitResult (Game|Player|GetHitResultUnderCursorbyChannel "TraceTypeQuery3" true)))))
    (:then
      (Class|ITFStockpiles|TargetTile(Message) (Variables|Default|GetSelectedActor) _asground_tile)
      (Variables|Default|SetControlMode "NewEnumerator0"))
    (:CastFailed
      (Development|PrintString "could not find tile")
      (Variables|Default|SetControlMode "NewEnumerator1"))))

(fn CreateResourceUi
  (params (sourceBuilding :type Building%20Object%20Reference))
  (bind _uimain_refpc (Variables|Default|GetUIMain_RefPC))
  (Widget|Panel|ClearChildren (Variables|/Game/UserInterfaces/UI_main.UI_Main_C|GetScrollBox_25 _uimain_refpc))
  (Widget|SetVisibility (Variables|/Game/UserInterfaces/UI_main.UI_Main_C|GetHorizontalBox_Resources _uimain_refpc) "Visible")
  (bind _returnvalue (UserInterface|CreateWidget "/Game/UserInterfaces/data_containers/resource_display.resource_display_C" self))
  (Variables|/Game/UserInterfaces/data_containers/resource_display.resource_display_C|SetsourceBuilding _returnvalue sourceBuilding)
  (Variables|/Game/UserInterfaces/data_containers/resource_display.resource_display_C|SetdisplayType _returnvalue "NewEnumerator0")
  (Widget|Panel|AddChild (Variables|/Game/UserInterfaces/UI_main.UI_Main_C|GetScrollBox_25 (Variables|Default|GetUIMain_RefPC)) _returnvalue))

(fn GlobalClick
  (bind _hitresult (Game|Player|GetHitResultUnderCursorbyChannel "TraceTypeQuery3" true))
  (bind (_bblockinghit _binitialoverlap _time _location _impactpoint _normal _impactnormal _physmat _hitactor) (Collision|BreakHitResult _hitresult))
  (bind (_x _y) (Math|Vector|BreakVector _location))
  (Utilities|IsValid (Variables|Default|GetUIGlobal)
    (:Is%20Valid
      (Variables|/Game/UserInterfaces/LandingSelection/UI_Global.UI_Global_C|Setloc_y (Variables|Default|GetUIGlobal) _y)
      (Variables|/Game/UserInterfaces/LandingSelection/UI_Global.UI_Global_C|Setloc_x (Variables|Default|GetUIGlobal) _x)
      (bind _asgi_main (Utilities|Casting|CastToGI_main (Game|GetGameInstance)))
      (Variables|/Game/Blueprints/GI_main.GI_main_C|SetLatitude _asgi_main (/ _y 1e+01))
      (Variables|/Game/Blueprints/GI_main.GI_main_C|SetLongitude _asgi_main (/ _x 1e+01))
      (Development|PrintString (Utilities|String|ToString(Vector) _location)))
    (:Is%20Not%20Valid
      (bind _returnvalue (UserInterface|CreateWidget "/Game/UserInterfaces/LandingSelection/UI_Global.UI_Global_C" self))
      (bind _output_get (Variables|Default|SetUIGlobal _returnvalue))
      (Variables|/Game/UserInterfaces/LandingSelection/UI_Global.UI_Global_C|Setcontroller _returnvalue 0)
      (UserInterface|Viewport|AddtoViewport _returnvalue 0)))
  (Variables|Default|SetControlMode "NewEnumerator6")
  (Utilities|Casting|CastToGroundTile _hitactor
    (:then
      (Development|PrintString "landed")
      (Variables|Default|SetControlMode "NewEnumerator0")
      (Widget|RemovefromParent _output_get)
      (Utilities|MainUiControl))
    (:CastFailed
      (Development|PrintString "in orbit"))))

(fn SpawnHUD
  (Utilities|MainUiControl))

(fn ClearUi
  (Utilities|ClearStockpileUI))